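; Spore is an enemy pawn that roams the navmesh, chases pawns it sees and explodes.
; Pawn sensing sets a flag that Tick uses to repeat the chase, otherwise moving to random nearby points after a delay.
; Player overlap with the detonation sphere or depleted health triggers falloff radial damage, effects and destruction.
; Damage from other Spores is briefly delayed, staggering chain explosions, and the construction script sizes both spheres.
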(event OnSeePawn(PawnSensing)
  (params (Pawn :type Pawn%20Object%20Reference))
  (Variables|Default|SetcharacterSeen true)
  (AI|AIMoveTo self "0, 0, 0" Pawn 5.0 true
    (:then
      (Variables|Default|SetcharacterSeen false))))

(event OnComponentBeginOverlap(DetCB)
  (params (OverlappedComponent :type Primitive%20Component%20Object%20Reference) (OtherActor :type Actor%20Object%20Reference) (OtherComp :type Primitive%20Component%20Object%20Reference) (OtherBodyIndex :type Integer) (bFromSweep :type Boolean) (SweepResult :type Hit%20Result%20Structure%20%28by%20ref%29))
  (bind _returnvalue (Transformation|GetActorLocation))
  (Utilities|Casting|CastToPlayer OtherActor)
  (Effects|SpawnEmitteratLocation "/Game/StarterContent/Particles/P_Explosion.P_Explosion" _returnvalue)
  (Class|GameplayStatics|ApplyRadialDamagewithFalloff 25.0 1e+01 _returnvalue (Variables|Default|GetDetRange) (Variables|Default|GetBlastRadius) 1.0 "/Script/Engine.DamageType" 0 self 0 "ECC_Visibility")
  (Audio|PlaySoundatLocation "/Game/StarterContent/Audio/Explosion02.Explosion02" _returnvalue)
  (Actor|DestroyActor))

(event EventTick
  (params (DeltaSeconds :type Float%20%28single-precision%29))
  (bind _self self)
  (if (Variables|Default|GetcharacterSeen)
    (AI|AIMoveTo _self "0, 0, 0" (stale OnSeePawn(PawnSensing) Pawn) 5.0 true
      (:then
        (Variables|Default|SetcharacterSeen false)))
    (else
      (Utilities|FlowControl|Delay 5.0)
      (AI|AIMoveTo _self (Class|NavigationSystem|GetRandomPointinNavigableRadius (Transformation|GetActorLocation) 1e+03) 0 5.0 true))))

(event Game|Damage|EventAnyDamage
  (params (Damage :type Float%20%28single-precision%29) (DamageType :type Damage%20Type%20Object%20Reference) (InstigatedBy :type Controller%20Object%20Reference) (DamageCauser :type Actor%20Object%20Reference))
  (bind _returnvalue (Transformation|GetActorLocation))
  (Utilities|Casting|CastToSpore DamageCauser
    (:then
      (Utilities|FlowControl|Delay 0.2))
    (:CastFailed
      _))
  (bind _output_get (Variables|Default|SetHealth (- (Variables|Default|GetHealth) Damage)))
  (if (<= _output_get 0.0)
    (Effects|SpawnEmitteratLocation "/Game/StarterContent/Particles/P_Explosion.P_Explosion" _returnvalue)
    (Class|GameplayStatics|ApplyRadialDamagewithFalloff 25.0 1e+01 _returnvalue (Variables|Default|GetDetRange) (Variables|Default|GetBlastRadius) 1.0 "/Script/Engine.DamageType" 0 self 0 "ECC_Visibility")
    (Audio|PlaySoundatLocation "/Game/StarterContent/Audio/Explosion02.Explosion02" _returnvalue)
    (Actor|DestroyActor)))

(fn ConstructionScript
  (Components|Sphere|SetSphereRadius (Variables|Default|GetExplodeCB) (Variables|Default|GetBlastRadius) true)
  (Components|Sphere|SetSphereRadius (Variables|Default|GetDetCB) (Variables|Default|GetDetRange) true))