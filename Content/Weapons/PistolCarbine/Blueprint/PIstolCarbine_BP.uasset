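; Pistol carbine weapon that a Player picks up by overlap and can fire.
; On overlap it snaps to the PistolHolster socket and registers as the player's Pistol, unless one is already carried.
; Fire calls Reload when out of ammo; otherwise it spawns a projectile and sound at BarrelEnd, then re-calls itself after a WeaponStats.ROF delay while Firing holds.
; Ammo is not decremented here, and GetWeaponStats is an empty stub.
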(event EventBeginPlay)

(event Collision|EventActorBeginOverlap
  (params (OtherActor :type Actor%20Object%20Reference))
  ;[1 1 1] If overlapped by Player, Check if pistol is carried
  (bind _asplayer (Utilities|Casting|CastToPlayer OtherActor))
  (if (not (Utilities|IsValid (Variables|/Game/Character/Bluprints/Player.Player_C|GetPistol _asplayer)))
    ;[1 1 1] If no pistol carried
    (Transformation|AttachComponentToComponent (Variables|/Game/Character/Bluprints/Player.Player_C|GetPlayerCharacter _asplayer) "PistolHolster" "SnapToTarget" "SnapToTarget" "SnapToTarget" true)
    (Variables|/Game/Character/Bluprints/Player.Player_C|SetPistol _asplayer self)))

(event EventFire
  (bind _pistol (Variables|Weapon|GetPistol))
  (bind _returnvalue (Transformation|GetSocketTransform _pistol "BarrelEnd" "RTS_World"))
  (if (<= (Variables|Default|GetAmmo) 0)
    (CallFunction|Reload)
    (else
      (Game|SpawnActorfromClass "/Game/FirstPersonBP/Blueprints/FirstPersonProjectile.FirstPersonProjectile_C" _returnvalue "Undefined" 0 (Variables|Actor|GetInstigator))
      (Audio|PlaySoundatLocation "/Game/FirstPersonBP/Audio/FirstPerson_WeaponFire.FirstPerson_WeaponFire" (.Location (Math|Transform|BreakTransform _returnvalue)))
      (Utilities|FlowControl|Delay (/ (.ROF (Utilities|Struct|BreakWeapon_S (Variables|Default|GetWeaponStats))) 1.0))
      (if (Variables|Default|GetFiring)
        (CallFunction|Fire)))))

(fn ConstructionScript)

(fn GetWeaponStats
  (return ""))